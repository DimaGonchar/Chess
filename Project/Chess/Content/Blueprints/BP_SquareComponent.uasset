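; BP_SquareComponent is a board square component meant to move the BP_BlackRook actor to a clicked square.
; OnSquareChoosed stores the clicked square's location and sets Move if the Moved flag is set.
; Disconnected logic would bind that handler, find the rook, interpolate it toward the stored location and set Moved on reaching this component's location.
; BeginPlay and Tick are empty, so none of that logic runs.
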(event Custom|OnSquareChoosed
  (params (TouchedComponent :type Primitive%20Component%20Object%20Reference) (ButtonPressed :type Key%20Structure :default "None"))
  (bind _asbp_square_component (Utilities|Casting|CastToBP_SquareComponent TouchedComponent))
  (Variables|Default|SetLoaction (Transformation|GetWorldLocation _asbp_square_component))
  (if (Variables|Default|Getmoved)
    (Variables|Default|Setmove true)))

(event EventBeginPlay)

(event EventTick
  (params (DeltaSeconds :type Float%20%28single-precision%29)))