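; BP_Board is a game board where a clicked shape can be moved to a clicked square.
; BeginPlay calls Init if the board is not yet initialized, then binds click handlers on every shape and square.
; Clicking a shape stores it as current and clears the target; clicking a square stores its world location as the target.
; Tick eases the current shape there with VInterpTo, using a zero vector as the idle sentinel.
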(event Custom|ChoosedSquare
  (params (TouchedComponent :type Primitive%20Component%20Object%20Reference) (ButtonPressed :type Key%20Structure :default "None"))
  (bind _assquare_component (Utilities|Casting|CastToSquareComponent TouchedComponent))
  (Variables|Default|SetSquareLocation (Transformation|GetWorldLocation _assquare_component)))

(event Custom|ShapesChoosed
  (params (TouchedActor :type Actor%20Object%20Reference) (ButtonPressed :type Key%20Structure :default "None"))
  (bind _asshape (Utilities|Casting|CastToShape TouchedActor))
  (Variables|Default|SetCurrentShape _asshape)
  (Variables|Default|SetSquareLocation "0, 0, 0"))

(event EventBeginPlay
  (if (Class|Board|GetIsBoardInited)
    _
    (else
      (Class|Board|Init)))
  (for _array_element (Class|Board|GetShapes)
    (EventDispatchers|AssignOnClicked _array_element (delegate Custom|ShapesChoosed)))
  (for _array_element_2 (Class|Board|GetSquares)
    (EventDispatchers|AssignOnClicked _array_element_2 (delegate Custom|ChoosedSquare))))

(event Collision|EventActorBeginOverlap
  (params (OtherActor :type Actor%20Object%20Reference)))

(event EventTick
  (params (DeltaSeconds :type Float%20%28single-precision%29))
  (bind _currentshape (Variables|Default|GetCurrentShape))
  (if (Math|Vector|NotEqual(Vector) (Variables|Default|GetSquareLocation) "0, 0, 0" 0.0001)
    (Transformation|SetActorLocation _currentshape (Math|Interpolation|VInterpTo (Transformation|GetActorLocation _currentshape) (Variables|Default|GetSquareLocation) DeltaSeconds 3.0) false false)
    (if (Math|Vector|Equal(Vector) (Transformation|GetActorLocation _currentshape) (Variables|Default|GetSquareLocation) 0.0001)
      (Variables|Default|SetSquareLocation "0, 0, 0"))))

(fn ConstructionScript)