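; Controller that handles mouse selection of Shape actors and their SquareComponents, apparently for a board-style game.
; Left click increments a click counter and traces under the cursor; only on the first click does it store the hit Shape and square and flag them selected.
; GetLastObject and SetLastObject expose the last shape and square.
; Second-click and color-comparison logic is unfinished and disconnected, and nothing resets the click counter.
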(event EventBeginPlay)

(event EventTick
  (params (DeltaSeconds :type Float%20%28single-precision%29)))

(event Input|MouseEvents|LeftMouseButton
  (params (Key :type Key%20Structure :default "None"))
  (bind (_hitresult _returnvalue) (Game|Player|GetHitResultUnderCursorbyChannel "TraceTypeQuery1" true))
  (bind (_bblockinghit _binitialoverlap _time _distance _location _impactpoint _normal _impactnormal _physmat _hitactor _hitcomponent) (Collision|BreakHitResult _hitresult))
  (:Pressed
    (Math|Integer|IncrementInt (Variables|Default|GetCurrentClick)
      (:%20%20
        (if _returnvalue
          (Utilities|FlowControl|Sequence
            (:then_0
              (switch int (Variables|Default|GetCurrentClick)
                (:1
                  (Utilities|FlowControl|Sequence
                    (:then_0
                      (bind _asshape (Utilities|Casting|CastToShape _hitactor))
                      (Variables|Default|SetSelectableShape _asshape)
                      (Variables|Default|SetShapeSelectabled true))
                    (:then_1
                      (bind _assquare_component (Utilities|Casting|CastToSquareComponent _hitcomponent))
                      (Variables|Default|SetSelectableSquare _assquare_component)
                      (Variables|Default|SetSquareSelectabled true))))))))))))

(fn ConstructionScript)

(fn GetLastObject
  (return (Variables|Default|GetLastShape) (Variables|Default|GetLastSquare)))

(fn SetLastObject
  (params (InShape :type Shape%20Object%20Reference%20%28by%20ref%29) (InSquare :type Square%20Component%20Object%20Reference%20%28by%20ref%29))
  (Variables|Default|SetLastShape InShape)
  (Variables|Default|SetLastSquare InSquare))